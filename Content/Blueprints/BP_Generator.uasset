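; BP_Generator is an interactable generator actor that the player switches on through a keypad widget.
; Its sphere overlap enables input and allows interaction, and pressing E while it is off opens WBP_GeneratorKeypad with a self-reference, UI focus and mouse cursor.
; The TurnOnGenerator event, not called within this graph, marks it on and turns its status light green.
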(event OnComponentBeginOverlap(Sphere)
  (params (OverlappedComponent :type Primitive%20Component%20Object%20Reference) (OtherActor :type Actor%20Object%20Reference) (OtherComp :type Primitive%20Component%20Object%20Reference) (OtherBodyIndex :type Integer) (bFromSweep :type Boolean) (SweepResult :type Hit%20Result%20Structure%20%28by%20ref%29))
  (Input|EnableInput (Game|GetPlayerController 0))
  (bind _output_get (Variables|Default|SetCanInteract true)))

(event OnComponentEndOverlap(Sphere)
  (params (OverlappedComponent :type Primitive%20Component%20Object%20Reference) (OtherActor :type Actor%20Object%20Reference) (OtherComp :type Primitive%20Component%20Object%20Reference) (OtherBodyIndex :type Integer))
  (Variables|Default|SetCanInteract false))

(event Custom|TurnOnGenerator
  (Variables|Default|SetIsGeneratorOn true)
  (Rendering|Components|Light|SetLightColor (Variables|Default|GetGeneratorStatusLight) "(R=0.000000,G=1.000000,B=0.000000,A=1.000000)" true))

(event EventBeginPlay)

(event Collision|EventActorBeginOverlap
  (params (OtherActor :type Actor%20Object%20Reference)))

(event EventTick
  (params (DeltaSeconds :type Float%20%28single-precision%29)))

(event Input|KeyboardEvents|E
  (params (Key :type Key%20Structure :default "None"))
  (bind _returnvalue (Game|GetPlayerController 0))
  (:Pressed
    (if (stale OnComponentBeginOverlap(Sphere) _output_get)
      (if (not (Variables|Default|GetIsGeneratorOn))
        (bind _returnvalue_2 (UserInterface|CreateWidget "/Game/Blueprints/WBP_GeneratorKeypad.WBP_GeneratorKeypad_C"))
        (Variables|/Game/Blueprints/WBP_GeneratorKeypad.WBP_GeneratorKeypad_C|SetGeneratorRef _returnvalue_2 self)
        (UserInterface|Viewport|AddtoViewport _returnvalue_2 0)
        (Input|SetInputModeGameandUI _returnvalue _returnvalue_2 "DoNotLock" true false)
        (Variables|/Script/Engine.PlayerController|SetbShowMouseCursor _returnvalue true)))))

(fn ConstructionScript)